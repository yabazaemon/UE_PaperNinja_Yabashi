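; BP_Pickup is a pickup actor that player-controlled pawns collect by overlapping it, ignoring AI-controlled pawns.
; On overlap it asks CanbeObtained, which by default passes only when the pawn's lifespan is zero.
; On success it runs the empty Obtainedmpl event, apparently a hook for child classes, then fires the OnObtained dispatcher and destroys itself.
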(event Custom|Obtainedmpl
  (params (Pawn :type Pawn%20Object%20Reference) (Player%20Controller] :type Player%20Controller%20Object%20Reference)))

(event EventBeginPlay)

(event Collision|EventActorBeginOverlap
  (params (OtherActor :type Actor%20Object%20Reference))
  ;[1 1 1] コントールしているのがAIか人間か判断
  (bind _asポーン (Utilities|Casting|CastToPawn OtherActor))
  (bind _asプレイヤーコントローラー (Utilities|Casting|CastToPlayerController (Pawn|GetController _asポーン)))
  (if (CallFunction|CanbeObtained _asポーン _asプレイヤーコントローラー)
    (CallFunction|Obtainedmpl _asポーン _asプレイヤーコントローラー)
    (Default|CallOnObtained)
    (Actor|DestroyActor)))

(event EventTick
  (params (DeltaSeconds :type Float%20%28single-precision%29)))

(fn ConstructionScript)

(fn CanbeObtained
  (params (Pawn :type Pawn%20Object%20Reference) (PlayerController :type Player%20Controller%20Object%20Reference))
  (return (== (Actor|GetLifeSpan Pawn) 0.0)))