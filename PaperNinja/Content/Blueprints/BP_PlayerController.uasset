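; Player controller that sets up Enhanced Input and automatically respawns the player character when it is destroyed.
; BeginPlay adds the default input mapping context to the local player subsystem.
; UnPossess waits one tick, asks the GameMode for a Player Start, then spawns a new BP_Player there and possesses it.
; The respawn has no condition, so any unpossess triggers it.
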(event EventBeginPlay
  (Input|AddMappingContext (PlayerController|LocalPlayerSubsystems|GetEnhancedInputLocalPlayerSubsystem) "/Game/Input/IMC_Default.IMC_Default" 0 "(bIgnoreAllPressedKeysUntilRelease=True,bForceImmediately=False,bNotifyUserSettings=False)"))

(event EventTick
  (params (DeltaSeconds :type Float%20%28single-precision%29)))

(event EventUnPossess
  (params (UnpossessedPawn :type Pawn%20Object%20Reference))
  (Utilities|FlowControl|DelayUntilNextTick)
  (bind _returnvalue (Game|SpawnActorfromClass "/Game/Blueprints/BP_Player.BP_Player_C" (Transformation|GetActorTransform (Class|GameModeBase|FindPlayerStart (Game|GetGameMode) self)) "Undefined" "MultiplyWithRoot" 0 0))
  (Pawn|Possess self _returnvalue))

(fn ConstructionScript)