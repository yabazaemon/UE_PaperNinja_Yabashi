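; BP_Turret is a turret actor that spins its barrel and fires BP_Bullet on a timed pattern, starting at BeginPlay.
; The FireControl timeline feeds the barrel's roll rate into a RotatingMovement component, and its Fire event track spawns each bullet at the Muzzle socket.
; Debug drawing shows a "Fire!" label in a timeline-driven color on each shot and an aim line from the muzzle every tick.
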(event EventBeginPlay
  (Components|Movement|SetUpdatedComponent (Variables|Default|GetRotatingMovement) (Variables|Default|GetBurrel))
  (bind (_direction _muzzlerolling _burret_collor) (Timeline|Fire%20Control Play)
    (:Update
      (Variables|/Script/Engine.RotatingMovementComponent|SetRotationRate (Variables|Default|GetRotatingMovement) (Math|Rotator|MakeRotator _muzzlerolling 0.0 0.0)))
    (:Fire
      (Rendering|Debug|DrawDebugString "0, 0, 0" "Fire!" self _burret_collor 0.2)
      (Game|SpawnActorfromClass "/Game/Blueprints/BP_Bullet.BP_Bullet_C" (CallFunction|GetMuzzleTransform) "Undefined" "MultiplyWithRoot" 0 0))))

(event Collision|EventActorBeginOverlap
  (params (OtherActor :type Actor%20Object%20Reference)))

(event EventTick
  (params (DeltaSeconds :type Float%20%28single-precision%29))
  (bind _returnvalue (CallFunction|GetMuzzleTransform))
  (bind (_location _rotation) (Math|Transform|BreakTransform _returnvalue))
  (bind _returnvalue_2 (Math|Vector|GetForwardVector _rotation))
  (bind (_start _end) (CallFunction|CalcRay _location _returnvalue_2 8e+02))
  (Rendering|Debug|DrawDebugLine _start _end "(R=0.000000,G=0.233631,B=1.000000,A=1.000000)" 0.0 2.0))

(fn ConstructionScript)

(fn GetMuzzleTransform
  (return (Transformation|GetSocketTransform (Variables|Debug|GetStaticMeshComponent) "Muzzle" "RTS_World")))